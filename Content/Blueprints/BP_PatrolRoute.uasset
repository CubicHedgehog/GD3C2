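; BP_PatrolRoute is a spline-based patrol route that supplies successive world-space points, ping-ponging along the spline.
; GetPatrolPointLocation calls IncrementPtrolPointIndex, then returns the spline point location at PatrolIndex.
; The increment steps PatrolIndex by Direction and reverses at either end.
; The upper check compares against the point count, so the index runs one past the last point before turning back.
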(event `IncrementPtrolPointIndex`
  (bind _patrolindex (`self.PatrolIndex`))
  (bind _patrolindex_2 (`self.PatrolIndex`))
  (set `self.PatrolIndex` (+ _patrolindex (`self.Direction`)))
  (if (>= _patrolindex (`SplineComponent.GetNumberOfSplinePoints` (`self.Spline`)))
    (set `self.Direction` (* (`self.Direction`) -1))
    (if (== _patrolindex_2 (`SplineComponent.GetNumberOfSplinePoints` (`self.Spline`)))
      (set `self.Direction` -1))
    (elif (<= _patrolindex_2 0)
      (set `self.Direction` 1))))

(fn `GetPatrolPointLocation`
  (returns (Location :type "Vector Structure"))
  (`self.IncrementPtrolPointIndex`)
  (return (`SplineComponent.GetLocationAtSplinePoint` (`self.Spline`) (`self.PatrolIndex`) "World")))

(fn `UserConstructionScript`)