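; BP_CameraDoor is a door that slides down when opened while the triggering player's camera blends to it.
; OpenDoor records the door in GMB_Coding2's LevelSave, then plays a timeline slide with camera shake and force feedback for both players.
; After a short hold, the view blends back to the passed target.
; quietOpen runs only the slide; pressure plate and load-state events are empty stubs.
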(event `quietOpen`
  (bind (_direction _newtrack_0) (`Timeline|Timeline_0`)
    (:`Update`
      (`SceneComponent.K2_SetRelativeLocation` (`self.Door`) (`KismetMathLibrary.VLerp` (0.0 0.0 150.0) (0.0 0.0 -155.0) _newtrack_0) false false))
    (:`Finished`
      (set `self.Closed` true))))

(event `PlatePressed2`)

(event `PlatePressed`
  (params (NewTarget :type "Actor Object Reference") (PlayerID :type Integer)))

(event `OpenDoor`
  (params (NewViewTarget :type "Actor Object Reference") (PlayerID :type Integer))
  (bind _returnvalue (`GameplayStatics.GetPlayerControllerFromID` PlayerID))
  (if (`self.Closed`)
    (bind _asgmb_coding_2 (cast `/Game/Blueprints/NewSaves/GMB_Coding2` (`GameplayStatics.GetGameMode`)))
    (`KismetArrayLibrary.Array_AddUnique` (`/Game/Blueprints/NewSaves/SG_LevelSave.OpenedDoors` (`/Game/Blueprints/NewSaves/GMB_Coding2.LevelSave` _asgmb_coding_2)) self)
    (`PlayerController.SetViewTargetWithBlend` _returnvalue self (`self.Blend Time`) "VTBlend_Cubic" 0.0 true)
    (`KismetSystemLibrary.Delay` (`self.Blend Time`))
    (`ForceFeedbackComponent.Play` (`self.ForceFeedback`) 0.0)
    (`PlayerController.ClientStartCameraShakeFromSource` (`GameplayStatics.GetPlayerController` 0) "/Game/Blueprints/CameraShake/CS_DoorSlideDown.CS_DoorSlideDown_C" (`self.CameraShakeSource`))
    (`PlayerController.ClientStartCameraShakeFromSource` (`GameplayStatics.GetPlayerController` 1) "/Game/Blueprints/CameraShake/CS_DoorSlideDown.CS_DoorSlideDown_C" (`self.CameraShakeSource`))
    (`PlayerController.K2_ClientPlayForceFeedback` (`GameplayStatics.GetPlayerController` 1) "/Game/Input/something/FFE_Door.FFE_Door" "None" false false false)
    (`PlayerController.K2_ClientPlayForceFeedback` (`GameplayStatics.GetPlayerController` 0) "/Game/Input/something/FFE_Door.FFE_Door" "None" false false false)
    (bind (_direction _newtrack_0) (`Timeline|Timeline`)
      (:`Update`
        (`SceneComponent.K2_SetRelativeLocation` (`self.Door`) (`KismetMathLibrary.VLerp` (0.0 0.0 150.0) (0.0 0.0 -155.0) _newtrack_0) false false))
      (:`Finished`
        (`KismetSystemLibrary.Delay` 2.0) ; waiting 2 seconds while the door opens
        (`PlayerController.SetViewTargetWithBlend` _returnvalue NewViewTarget (/ (`self.Blend Time`) 2.0) "VTBlend_Cubic" 0.0 false) ; shift camera back to player
        (set `self.Closed` true)))))

(event `LoadDoorState`)

(event `UnloadDoorState`)

(fn `UserConstructionScript`)