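; BP_NodeManager is an actor that spawns node actors, apparently as an unfinished prototype.
; On BeginPlay it spawns a BP_NodeInClass at its own location, stores it as LastNode and zeroes NodeIndex.
; SpawnNewNode prints a debug string and spawns the same class at a zero-extent random point, effectively the manager's location, then resets and increments NodeIndex.
; Notes mark the intended class as BP_Node and target assignment as still to add.
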(event `self.ReceiveBeginPlay`
  (bind _returnvalue (`|SpawnActorFromClass` "/Game/Blueprints/NodeStuff/BP_NodeInClass.BP_NodeInClass_C" (`KismetMathLibrary.MakeTransform` (`self.K2_GetActorLocation`)) "Undefined" "MultiplyWithRoot" null null))
  (set `self.LastNode` _returnvalue)
  (set `self.NodeIndex` 0))

(event `SpawnNewNode`
  (`KismetSystemLibrary.PrintString` "Hello")
  (`|SpawnActorFromClass` "/Game/Blueprints/NodeStuff/BP_NodeInClass.BP_NodeInClass_C" (`KismetMathLibrary.MakeTransform` (`KismetMathLibrary.RandomPointInBoundingBox` (`self.K2_GetActorLocation`))) "Undefined" "MultiplyWithRoot" null null) ; Class should by BP_Node
  (set `self.NodeIndex` 0) ; add target
  (`/Engine/EditorBlueprintResources/StandardMacros.IncrementInt` (`self.NodeIndex`)))

(fn `UserConstructionScript`)