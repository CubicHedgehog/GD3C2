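; GMB_Coding2 is a Game Mode that handles per-level saving, using the current level name as the save slot.
; On BeginPlay it loads or creates an SG_LevelSave, applies collected coins and moves the player to any non-zero saved location.
; Checkpoint stores a player transform and FinishedLevel clears it, both writing through SaveGame.
; A save that fails the cast is deleted without a replacement being created.
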(event `self.ReceiveBeginPlay`
  (bind _levelsave (`self.LevelSave`))
  (bind _playertransform_location (`KismetMathLibrary.BreakTransform` (`/Game/Blueprints/NewSaves/SG_LevelSave.PlayerTransform` _levelsave)))
  (`KismetSystemLibrary.PrintString` "Loaded into GMB_Coding2 Game Mode" true true (struct :`R` 0.987233 :`G` 0.435021 :`B` 1.0 :`A` 1.0) 20.0)
  ;[1 1 1] Comment
  (bind _returnvalue (`GameplayStatics.GetCurrentLevelName` true))
  (bind _returnvalue_2 (`GameplayStatics.DoesSaveGameExist` _returnvalue))
  (if _returnvalue_2
    (bind _returnvalue_3 (`GameplayStatics.LoadGameFromSlot` _returnvalue))
    (bind _assg_level_save (cast `/Game/Blueprints/NewSaves/SG_LevelSave` _returnvalue_3)
      (:`then`
        (bind _output_get (set `self.LevelSave` _assg_level_save))
        (`/Game/Blueprints/NewSaves/SG_LevelSave.LoadCollectedCoins` _output_get) ; change coins that have been collected
        (if (not (`KismetMathLibrary.EqualExactly_VectorVector` _playertransform_location))
          (`SceneComponent.K2_SetWorldTransform` (`Character.CapsuleComponent` (`GameplayStatics.GetPlayerCharacter` 0)) (`/Game/Blueprints/NewSaves/SG_LevelSave.PlayerTransform` _levelsave) false false)))
      (:`CastFailed`
        (`GameplayStatics.DeleteGameInSlot` _returnvalue)))
    (else
      (bind _returnvalue_4 (`GameplayStatics.CreateSaveGameObject` "/Game/Blueprints/NewSaves/SG_LevelSave.SG_LevelSave_C"))
      (set `self.LevelSave` _returnvalue_4))))

(event `SaveGame`
  (bind _returnvalue (`GameplayStatics.GetCurrentLevelName` true))
  (bind _returnvalue_2 (`GameplayStatics.SaveGameToSlot` (`self.LevelSave`) _returnvalue))
  (if _returnvalue_2
    (`KismetSystemLibrary.PrintString` "SAVED LEVEL")
    (else
      (`KismetSystemLibrary.PrintString` "COULD NOT SAVE LEVEL"))))

(fn `Checkpoint`
  (params (PlayerTransform :type "Transform Structure"))
  (set `/Game/Blueprints/NewSaves/SG_LevelSave.PlayerTransform` PlayerTransform (`self.LevelSave`))
  (`self.SaveGame`))

(fn `FinishedLevel`
  (set `/Game/Blueprints/NewSaves/SG_LevelSave.PlayerTransform` (struct) (`self.LevelSave`)) ; Reset player start location
  (`self.SaveGame`))

(fn `UserConstructionScript`)