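; Checkpoint actor that records a player save point when a BP_ThirdPersonCharacter overlaps its sphere.
; It passes GMB_Coding2's Checkpoint a transform built from a point above its Cube plus the player's rotation and scale, then activates its CheckpointSystem component.
; Unconnected leftover nodes for LastSavedLocation and a second activation never run.
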(event `self.Sphere.OnComponentBeginOverlap`
  (params (OverlappedComponent :type "PrimitiveComponent Object Reference") (OtherActor :type "Actor Object Reference") (OtherComp :type "PrimitiveComponent Object Reference") (OtherBodyIndex :type Integer) (bFromSweep :type Boolean) (SweepResult :type "HitResult Structure (by ref)"))
  (bind (_returnvalue_location _returnvalue_rotation _returnvalue_scale) (`KismetMathLibrary.BreakTransform` (`self.GetTransform` OtherActor)))
  (cast `/Game/ThirdPerson/Blueprints/BP_ThirdPersonCharacter` OtherActor)
  (bind _asgmb_coding_2 (cast `/Game/Blueprints/NewSaves/GMB_Coding2` (`GameplayStatics.GetGameMode`)))
  (`/Game/Blueprints/NewSaves/GMB_Coding2.Checkpoint` _asgmb_coding_2 (`KismetMathLibrary.MakeTransform` (+ (`SceneComponent.K2_GetComponentLocation` (`self.Cube`)) (0.0 0.0 100.0)) _returnvalue_rotation _returnvalue_scale))
  (`ActorComponent.Activate` (`self.CheckpointSystem`) true))

(fn `UserConstructionScript`)