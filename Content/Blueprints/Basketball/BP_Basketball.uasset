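; Basketball pickup that bounces on its own and is collected when the player overlaps its box.
; Each tick, a vertical line trace offset by ProximityDistance gates a random force, scaled per axis along the mesh's forward vector.
; Player overlap adds the ball to the GMB_Coding2 game mode's LevelSave.CollectedBalls, then destroys it.
; LoadCollectedStateBalls applies an emissive pink material to show collected state.
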(event `self.ReceiveTick`
  (params (DeltaSeconds :type "Float (single-precision)"))
  (bind _maxforcetobounce (`self.MaxForceToBounce`))
  (bind _minforcetobounce (`self.MinForceToBounce`))
  (bind _iscontact_ (`self.DetectGround` (`self.StaticMesh`))
    (:`Out`
      (if _iscontact_
        (`PrimitiveComponent.AddForce` (`self.StaticMesh`) (* (`SceneComponent.GetForwardVector` (`self.StaticMesh`)) (`KismetMathLibrary.MakeVector` (`KismetMathLibrary.RandomFloatInRange` _minforcetobounce _maxforcetobounce) (`KismetMathLibrary.RandomFloatInRange` _minforcetobounce _maxforcetobounce) (`KismetMathLibrary.RandomFloatInRange` _minforcetobounce _maxforcetobounce))) "None" true)))))

(event `self.Box.OnComponentBeginOverlap`
  (params (OverlappedComponent :type "PrimitiveComponent Object Reference") (OtherActor :type "Actor Object Reference") (OtherComp :type "PrimitiveComponent Object Reference") (OtherBodyIndex :type Integer) (bFromSweep :type Boolean) (SweepResult :type "HitResult Structure (by ref)"))
  (set `self.BallOverlap` true)
  (cast `/Game/ThirdPerson/Blueprints/BP_ThirdPersonCharacter` OtherActor) ; If player hits this
  (bind _asgmb_coding_2 (cast `/Game/Blueprints/NewSaves/GMB_Coding2` (`GameplayStatics.GetGameMode`))) ; Get GameMode we want
  (`KismetArrayLibrary.Array_AddUnique` (`/Game/Blueprints/NewSaves/SG_LevelSave.CollectedBalls` (`/Game/Blueprints/NewSaves/GMB_Coding2.LevelSave` _asgmb_coding_2)) self)
  (`self.K2_DestroyActor`))

(event `self.Box.OnComponentEndOverlap`
  (params (OverlappedComponent :type "PrimitiveComponent Object Reference") (OtherActor :type "Actor Object Reference") (OtherComp :type "PrimitiveComponent Object Reference") (OtherBodyIndex :type Integer))
  (set `self.BallOverlap` false))

(event `LoadCollectedStateBalls`
  (`PrimitiveComponent.SetMaterial` (`self.StaticMesh`) 0 "/Game/Materials/MI_EmissivePink.MI_EmissivePink")
  (`KismetSystemLibrary.PrintString` "CollectedStateLoaded"))

(fn `UserConstructionScript`)