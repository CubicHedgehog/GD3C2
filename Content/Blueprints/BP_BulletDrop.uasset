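; Bullet-drop test actor that fires a simulated projectile from its Arrow's location every two seconds, starting at BeginPlay.
; ReallyCoolCalculator steps the path with chained line traces, adding gravity to velocity each step, up to SimFrequency steps.
; The first hit prints the actor and location, plays a sound and spawns fire, then start and velocity reset.
; Debug drawing and a built-in PredictProjectilePath alternative are left disconnected.
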(event `ReallyCoolCalculator`
  (set `self.End` (+ (`self.Start`) (/ (`self.Velocity`) (`KismetMathLibrary.MakeVector` (`self.Sim Frequency`) 1.0 1.0))))
  (for _ (range 1 (+ (`KismetMathLibrary.FTrunc` (`self.Sim Frequency`)) 1))
    (bind (_outhit _returnvalue) (`KismetSystemLibrary.LineTraceSingleByProfile` (`self.Start`) (`self.End`) "BlockAll"))
    (if _returnvalue
      (bind (_bblockinghit _binitialoverlap _time _distance _location _impactpoint _normal _impactnormal _physmat _hitactor) (`GameplayStatics.BreakHitResult` _outhit))
      (`KismetSystemLibrary.PrintString` (`KismetStringLibrary.Concat_StrStr` "Hit Actor: " (`KismetSystemLibrary.GetDisplayName` _hitactor) " \nLocation: " (`KismetStringLibrary.Conv_VectorToString` _impactpoint)))
      (`GameplayStatics.PlaySoundAtLocation` "/Game/Audio/bleepbloops.bleepbloops" _impactpoint (struct) 1.0 1.0 0.0 null null null null)
      (`GameplayStatics.SpawnEmitterAtLocation` "/Game/Fantastic_Village_Pack/effects/PS_FX_fire_1.PS_FX_fire_1" _impactpoint)
      (break)
      (else
        (set `self.Start` (`self.End`))
        (set `self.Velocity` (+ (`self.Velocity`) (`KismetMathLibrary.MakeVector` 0.0 0.0 (/ -980.0 (`KismetMathLibrary.Square` (`self.Sim Frequency`))))))
        (set `self.End` (+ (`self.Start`) (/ (`self.Velocity`) (`KismetMathLibrary.MakeVector` (`self.Sim Frequency`) 1.0 1.0)))))))
  (set `self.Start` (`SceneComponent.K2_GetComponentLocation` (`self.Arrow`)))
  (set `self.Velocity` (400.0 0.0 0.0)))

(event `self.ReceiveBeginPlay`
  (set `self.Start` (`SceneComponent.K2_GetComponentLocation` (`self.Arrow`)))
  (`|ExecutionSequence` :!label _label
    (:`then_0`
      (`self.ReallyCoolCalculator`))
    (:`then_1`
      (`KismetSystemLibrary.Delay` 2.0)
      (goto _label))))

(fn `UserConstructionScript`)