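; BP_GoToNextLevel is a level exit trigger that sends the player on to a configurable destination level.
; When BP_ThirdPersonCharacter overlaps its sphere, it calls FinishedLevel on the GMB_Coding2 game mode, then opens levels.
; It calls open-level by the name "None" and by DestinationLevel before the validity check, which opens DestinationLevel again or prints a missing-destination message.
; A current-level name comparison is left unconnected.
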(event `self.Sphere.OnComponentBeginOverlap`
  (params (OverlappedComponent :type "PrimitiveComponent Object Reference") (OtherActor :type "Actor Object Reference") (OtherComp :type "PrimitiveComponent Object Reference") (OtherBodyIndex :type Integer) (bFromSweep :type Boolean) (SweepResult :type "HitResult Structure (by ref)"))
  (cast `/Game/ThirdPerson/Blueprints/BP_ThirdPersonCharacter` OtherActor)
  (bind _asgmb_coding_2 (cast `/Game/Blueprints/NewSaves/GMB_Coding2` (`GameplayStatics.GetGameMode`)))
  (`/Game/Blueprints/NewSaves/GMB_Coding2.FinishedLevel` _asgmb_coding_2)
  (`GameplayStatics.OpenLevel` "None")
  (`GameplayStatics.OpenLevelBySoftObjectPtr` (`self.DestinationLevel`))
  (bind _destinationlevel (`self.DestinationLevel`)
    (:`then`
      (`GameplayStatics.OpenLevelBySoftObjectPtr` _destinationlevel))
    (:`else`
      (`KismetSystemLibrary.PrintString` "No destination level selected"))))

(fn `UserConstructionScript`)